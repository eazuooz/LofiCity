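; BP_Cable is a spline-driven cable actor that builds its mesh in the construction script.
; Each spline segment gets a spline mesh fitted to its points and tangents.
; Three material slots per segment get dynamic instances, with start and end parameters holding the segment's distances measured back from the spline's end.
; When CapBeginning is set, it also adds beginning and end cap meshes oriented along the spline tangents.
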(fn `UserConstructionScript`
  (locals (NewVar :type Boolean))
  (bind _spline1 (`self.Spline1`))
  (bind _returnvalue (`SplineComponent.GetSplineLength` _spline1))
  (bind (_location _tangent) (`SplineComponent.GetLocationAndTangentAtSplinePoint` _spline1 0 "Local"))
  (for _index (range (+ (- (`SplineComponent.GetNumberOfSplinePoints` _spline1) 2) 1))
    (bind _returnvalue_2 (`AddComponent|NODE_AddSplineMeshComponent-0`))
    (bind _returnvalue_3 (`PrimitiveComponent.CreateDynamicMaterialInstance` _returnvalue_2 0 null "None"))
    (set `self.Dy_Mat` _returnvalue_3)
    (bind _returnvalue_4 (+ _index 1))
    (bind _returnvalue_5 (- _returnvalue (`SplineComponent.GetDistanceAlongSplineAtSplinePoint` _spline1 _returnvalue_4)))
    (`MaterialInstanceDynamic.SetScalarParameterValue` _returnvalue_3 "start" _returnvalue_5)
    (bind _returnvalue_6 (- _returnvalue (`SplineComponent.GetDistanceAlongSplineAtSplinePoint` _spline1 _index)))
    (`MaterialInstanceDynamic.SetScalarParameterValue` _returnvalue_3 "end" _returnvalue_6)
    (bind _returnvalue_7 (`PrimitiveComponent.CreateDynamicMaterialInstance` _returnvalue_2 1 null "None"))
    (set `self.Dy_Mat02` _returnvalue_7)
    (`MaterialInstanceDynamic.SetScalarParameterValue` _returnvalue_7 "start" _returnvalue_5)
    (`MaterialInstanceDynamic.SetScalarParameterValue` _returnvalue_7 "end" _returnvalue_6)
    (bind _returnvalue_8 (`PrimitiveComponent.CreateDynamicMaterialInstance` _returnvalue_2 2 null "None"))
    (set `self.Dy_mat03` _returnvalue_8)
    (`MaterialInstanceDynamic.SetScalarParameterValue` _returnvalue_8 "start" _returnvalue_5)
    (`MaterialInstanceDynamic.SetScalarParameterValue` _returnvalue_8 "end" _returnvalue_6)
    (`SceneComponent.K2_AttachTo` _returnvalue_2 (`self.spline_mesh`) "None" "KeepRelativeOffset" true)
    (bind (_location_2 _tangent_2) (`SplineComponent.GetLocationAndTangentAtSplinePoint` _spline1 _index "Local"))
    (bind (_location_3 _tangent_3) (`SplineComponent.GetLocationAndTangentAtSplinePoint` _spline1 _returnvalue_4 "Local"))
    (`SplineMeshComponent.SetStartAndEnd` _returnvalue_2 _location_2 _tangent_2 _location_3 _tangent_3 true))
  (if (`self.Cap Beginning?`)
    (bind _returnvalue_9 (`AddComponent|NODE_AddStaticMeshComponent-1`))
    (`StaticMeshComponent.SetStaticMesh` _returnvalue_9 (`self.Cap Beginning`))
    (`SceneComponent.K2_SetRelativeLocation` _returnvalue_9 _location false false)
    (`SceneComponent.K2_SetRelativeRotation` _returnvalue_9 (`KismetMathLibrary.Conv_VectorToRotator` _tangent) false false)
    (bind _returnvalue_10 (`AddComponent|NODE_AddStaticMeshComponent-0`))
    (`StaticMeshComponent.SetStaticMesh` _returnvalue_10 (`self.Cap End`))
    (`SceneComponent.K2_SetRelativeLocation` _returnvalue_10 _location_2 false false)
    (`SceneComponent.K2_SetRelativeRotation` _returnvalue_10 (`KismetMathLibrary.Conv_VectorToRotator` _tangent_2) false false)))